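; Game mode for Toon Tanks that shows the menu, start and end screens through the StartGame and GameOver events.
; StartGame branches on the level name: MainMenu gets the menu widget with UI-only input, a visible cursor and IsInMainMenu set.
; Other levels get a start widget fed StartDelay as its timer, with the cursor hidden.
; GameOver passes the win result to the end-game widget.
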(event EventBeginPlay)

(event EventTick
  (params (DeltaSeconds :type Float%20%28single-precision%29)))

(event EventStartGame
  (bind _returnvalue (Game|GetPlayerController 0))
  (Variables|Default|SetIsInMainMenu false)
  (bind _returnvalue_2 (Game|GetCurrentLevelName true))
  (if (Utilities|Enum|Equal(Enum) _returnvalue_2 "MainMenu")
    (bind _returnvalue_3 (UserInterface|CreateWidget "/Game/Blueprints/Widgets/WBP_MainMenuWidget.WBP_MainMenuWidget_C"))
    (UserInterface|Viewport|AddtoViewport _returnvalue_3 0)
    (Variables|Default|SetIsInMainMenu true)
    (Input|SetInputModeUIOnly _returnvalue _returnvalue_3 "LockOnCapture")
    (Variables|/Script/Engine.PlayerController|SetbShowMouseCursor _returnvalue true)
    (else
      (bind _returnvalue_4 (UserInterface|CreateWidget "/Game/Blueprints/Widgets/WBP_StartGameWidget.WBP_StartGameWidget_C" 0 (Variables|Default|GetStartDelay)))
      (UserInterface|Viewport|AddtoViewport _returnvalue_4 0)
      (Variables|/Script/Engine.PlayerController|SetbShowMouseCursor (Game|GetPlayerController 0) false))))

(event EventGameOver
  (params (bWonGame :type Boolean))
  (bind _returnvalue (UserInterface|CreateWidget "/Game/Blueprints/Widgets/WBP_EndGameWidget.WBP_EndGameWidget_C" 0 bWonGame))
  (UserInterface|Viewport|AddtoViewport _returnvalue 0))

(fn ConstructionScript)